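; BP_ThrowableWeapons is a thrown projectile that damages AI on contact.
; BeginPlay sets its damage from the IsMonarchProjectile flag, with Monarch projectiles dealing less.
; Any sphere overlap applies damage if the actor is BP_AI, then spawns BP_ThrowableAmmunition in its place, passing the Monarch flag, and destroys the projectile.
; Bounce logic and its damage bonus are present but never run.
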(event `self.ReceiveBeginPlay`
  (if (`self.bIsMonarchProjectile`)
    (set `self.Damage` 5.0)
    (else
      (set `self.Damage` 15.0))))

(event `self.Sphere.OnComponentBeginOverlap`
  (params (OverlappedComponent :type "PrimitiveComponent Object Reference") (OtherActor :type "Actor Object Reference") (OtherComp :type "PrimitiveComponent Object Reference") (OtherBodyIndex :type Integer) (bFromSweep :type Boolean) (SweepResult :type "HitResult Structure (by ref)"))
  (bind (_asbp_ai _bsuccess) (cast `/Game/Core/AI/BP_AI` OtherActor :!pure true))
  (if _bsuccess
    (`GameplayStatics.ApplyDamage` _asbp_ai (`self.Damage`)))
  (`|SpawnActorFromClass` "/Game/Core/Ammunations/BP_ThrowableAmmunition.BP_ThrowableAmmunition_C" (`SceneComponent.K2_GetComponentToWorld` (`self.DefaultSceneRoot`)) "Undefined" "MultiplyWithRoot" null (`self.bIsMonarchProjectile`) null)
  (`self.K2_DestroyActor`))

(fn `UserConstructionScript`)