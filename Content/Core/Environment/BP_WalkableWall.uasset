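; BP_WalkableWall is a wall that carries the third-person character along a climb path when they touch it while not in the air.
; Overlapping the Box starts the Climbing timeline, whose UpWeGo value maps to a distance along the Spline.
; Each update moves the character's capsule to that world point with a sweep.
; The construction script multiplies the Cube's vertical scale by Height.
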(event `self.Box.OnComponentBeginOverlap`
  (params (OverlappedComponent :type "PrimitiveComponent Object Reference") (OtherActor :type "Actor Object Reference") (OtherComp :type "PrimitiveComponent Object Reference") (OtherBodyIndex :type Integer) (bFromSweep :type Boolean) (SweepResult :type "HitResult Structure (by ref)"))
  (bind _spline (`self.Spline`))
  (bind _asbp_third_person_character (cast `/Game/ThirdPerson/Blueprints/BP_ThirdPersonCharacter` OtherActor))
  (if (not (`/Game/ThirdPerson/Blueprints/BP_ThirdPersonCharacter.bInAir` _asbp_third_person_character))
    (bind (_direction _upwego) (`Timeline|Climbing` :!via `PlayFromStart`)
      (:`Update`
        (`SceneComponent.K2_SetWorldLocation` (`Character.CapsuleComponent` _asbp_third_person_character) (`SplineComponent.GetLocationAtDistanceAlongSpline` _spline (`KismetMathLibrary.Lerp` 0.0 (`SplineComponent.GetSplineLength` _spline) _upwego) "World") true false)))))

(fn `UserConstructionScript`
  (bind _cube (`self.Cube`))
  (bind (_returnvalue_x _returnvalue_y _returnvalue_z) (`KismetMathLibrary.BreakVector` (`SceneComponent.K2_GetComponentScale` _cube)))
  (`SceneComponent.SetWorldScale3D` _cube (`KismetMathLibrary.MakeVector` _returnvalue_x _returnvalue_y (* _returnvalue_z (`self.Height`)))))